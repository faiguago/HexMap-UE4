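; Player controller for painting a hex map with the mouse, setting cell color and elevation.
; BeginPlay shows the cursor and disables move and look input, and the left mouse button sets a pressed flag.
; While pressed, Tick traces under the cursor, prints the hex coordinates and updates the HexGrid cell there.
; Color and scaled elevation come from the hex map widget on BP_Hud.
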(event `self.ReceiveBeginPlay`
  ;[1 1 1] Initial Setup
  (set `self.bShowMouseCursor` true)
  (`self.SetIgnoreMoveInput` true)
  (`self.SetIgnoreLookInput` true))

(event `Key|LeftMouseButton`
  (params (Key :type "Key Structure"))
  ;[1 1 1] Left Mouse Input
  (:`Pressed`
    (set `self.bIsMousePressed` true))
  (:`Released`
    (set `self.bIsMousePressed` false)))

(event `self.ReceiveTick`
  (params (DeltaSeconds :type "Float (single-precision)"))
  (bind (_bblockinghit _binitialoverlap _time _distance _location) (`GameplayStatics.BreakHitResult` (`self.GetHitResultUnderCursorByChannel` "TraceTypeQuery3")))
  ;[1 1 1] Update Cells
  (if (`self.bIsMousePressed`)
    (bind _returnvalue (`HexLibrary.HexCoordinatesFromPosition` _location))
    (`KismetSystemLibrary.PrintString` (`KismetStringLibrary.Conv_VectorToString` _returnvalue) true true (struct :`G` 0.66 :`B` 1.0 :`A` 1.0) DeltaSeconds)
    (bind _asbp_hud (cast `/Game/_BP/BP_Hud` (`self.GetHUD`)))
    (bind _uw_hexmap (`/Game/_BP/BP_Hud.UW_HexMap` _asbp_hud))
    (`HexGrid.UpdateCell` (`self.HexGrid`) _location (`/Game/_BP/UI/WP_HexMapEditor.ActiveColor` _uw_hexmap) (* (`/Game/_BP/UI/WP_HexMapEditor.CurrentElevation` _uw_hexmap) 5.0))))

(fn `UserConstructionScript`)